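; BP_Guts is the playable Guts character, with camera-relative movement, mouse look and combat handled through TPCombatComponent.
; On BeginPlay the combat component equips BP_Dragonslayer in the RightHandWeapon slot and fully heals the character.
; Forward input follows the camera's forward vector flattened to the horizontal plane, and strafing follows its right vector.
; Left mouse button asks the combat component to use the first entry in CharacterAbilities.
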(event EventBeginPlay
  (Class|TPCombatComponent|EquipItem (Variables|Default|GetTPCombatComponent) "/TPCombat/Weapons/Greatswords/Dragonslayer/BP_Dragonslayer.BP_Dragonslayer_C" (Utilities|Name|MakeLiteralName "RightHandWeapon"))
  (Class|TPCombatComponent|FullHeal (Variables|Default|GetTPCombatComponent)))

(event Input|AxisEvents|InputAxisMoveForward
  (params (AxisValue :type Float%20%28single-precision%29))
  (bind _camera (Variables|Default|GetCamera))
  (bind _returnvalue (Math|Vector|GetForwardVector _camera))
  (Pawn|Input|AddMovementInput (Math|Vector|Normalize (Math|Vector|MakeVector (.x _returnvalue) (.y _returnvalue) 0.0) 0.001) AxisValue false))

(event Input|AxisEvents|InputAxisMoveRight
  (params (AxisValue :type Float%20%28single-precision%29))
  (Pawn|Input|AddMovementInput (Math|Vector|GetRightVector (Variables|Default|GetCamera)) AxisValue false))

(event Input|MouseEvents|MouseX
  (params (AxisValue :type Float%20%28single-precision%29))
  (Pawn|Input|AddControllerYawInput AxisValue))

(event Input|MouseEvents|MouseY
  (params (AxisValue :type Float%20%28single-precision%29))
  (Pawn|Input|AddControllerPitchInput AxisValue))

(event Input|MouseEvents|LeftMouseButton
  (params (Key :type Key%20Structure :default "None"))
  (:Pressed
    (Class|TPCombatComponent|TryUseAbility (Variables|Default|GetTPCombatComponent) (Utilities|Array|Get(acopy) (Variables|Default|GetCharacterAbilities)))))

(fn ConstructionScript)